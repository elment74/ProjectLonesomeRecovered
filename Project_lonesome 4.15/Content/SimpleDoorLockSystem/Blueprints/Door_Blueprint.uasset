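; Interactive swinging door Blueprint that can be locked or fake until other code calls Unlock or ConvertToReal.
; An overlap trigger enables input and opens a Gate, so touch or the Use action works only nearby.
; A real, unlocked door rotates via a Timeline that plays or reverses, with a FlipFlop tracking the closed state.
; Locked and fake doors briefly show UMG messages created at BeginPlay, guarded by resettable DoOnce nodes.
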(event OnComponentBeginOverlap(Trigger1)
  (params (OverlappedComponent :type Primitive%20Component%20Object%20Reference) (OtherActor :type Actor%20Object%20Reference) (OtherComp :type Primitive%20Component%20Object%20Reference) (OtherBodyIndex :type Integer) (bFromSweep :type Boolean) (SweepResult :type Hit%20Result%20Structure%20%28by%20ref%29))
  ;[1 1 1] Door
  (Input|EnableInput (Game|GetPlayerController 0))
  (Utilities|FlowControl|Gate true) ; enters at Open
)

(event OnComponentEndOverlap(Trigger1)
  (params (OverlappedComponent :type Primitive%20Component%20Object%20Reference) (OtherActor :type Actor%20Object%20Reference) (OtherComp :type Primitive%20Component%20Object%20Reference) (OtherBodyIndex :type Integer))
  ;[1 1 1] Door
  (Input|DisableInput (Game|GetPlayerController 0))
  (Utilities|FlowControl|Gate true) ; enters at Close
)

(event Custom|Reset
  ;[1 1 1] Door
  (Utilities|FlowControl|DoOnce false) ; enters at Reset
)

(event Custom|Reset2
  ;[1 1 1] Door
  (Utilities|FlowControl|DoOnce false) ; enters at Reset
)

(event Custom|ConvertToReal
  ;[1 1 1] Convert fake door to real door
  (Variables|Default|SetFakeDoor false))

(event Custom|Unlock
  ;[1 1 1] Key Unlock
  (Variables|Default|SetLocked false))

(event EventBeginPlay
  (bind _returnvalue (UserInterface|CreateWidget "/Game/SimpleDoorLockSystem/UMG´s/NeedKeyText.NeedKeyText_C"))
  ;[1 1 1] Change the ZOrder to what ever you want
  (UserInterface|Viewport|AddtoViewport _returnvalue 0)
  (bind _returnvalue_2 (UserInterface|CreateWidget "/Game/SimpleDoorLockSystem/UMG´s/FakeDoorText.FakeDoorText_C"))
  ;[1 1 1] Change the ZOrder to what ever you want
  (UserInterface|Viewport|AddtoViewport _returnvalue_2 0))

(event Input|ActionEvents|InputActionUse
  (params (Key :type Key%20Structure :default "AnyKey"))
  ;[1 1 1] Door
  (:Pressed
    (Utilities|FlowControl|Gate true
      (:Exit
        (if (Variables|Default|GetFakeDoor)
          (Utilities|FlowControl|DoOnce false
            (:Completed
              (Widget|SetVisibility (Variables|/Game/SimpleDoorLockSystem/UMG´s/FakeDoorText.FakeDoorText_C|GetTextBox (stale EventBeginPlay _returnvalue_2)) "Visible")
              (Utilities|FlowControl|Delay 3.0)
              (Widget|SetVisibility (Variables|/Game/SimpleDoorLockSystem/UMG´s/FakeDoorText.FakeDoorText_C|GetTextBox (stale EventBeginPlay _returnvalue_2)) "Hidden")
              (CallFunction|Reset2)))
          (elif (Variables|Default|GetLocked)
            (Utilities|FlowControl|DoOnce false
              (:Completed
                (Rendering|Components|TextRender|SetText (Variables|/Game/SimpleDoorLockSystem/UMG´s/NeedKeyText.NeedKeyText_C|GetKeyText (stale EventBeginPlay _returnvalue)) "")
                (Widget|SetVisibility (Variables|/Game/SimpleDoorLockSystem/UMG´s/NeedKeyText.NeedKeyText_C|GetHorizontalBox_428 (stale EventBeginPlay _returnvalue)) "Visible")
                (Utilities|FlowControl|Delay 1.5)
                (Widget|SetVisibility (Variables|/Game/SimpleDoorLockSystem/UMG´s/NeedKeyText.NeedKeyText_C|GetHorizontalBox_428 (stale EventBeginPlay _returnvalue)) "Hidden")
                (CallFunction|Reset)))
            (elif (Variables|Default|GetClosed?)
              (bind _doorrotation (Timeline|Door%20Opening%20Animation Play)
                (:Update
                  (Transformation|SetRelativeRotation (Variables|Default|GetDoor) (Math|Rotator|MakeRotator 0.0 0.0 _doorrotation) false false))
                (:Finished
                  (Utilities|FlowControl|FlipFlop
                    (:A
                      (Variables|Default|SetClosed? false))
                    (:B
                      (Variables|Default|SetClosed? true)))))
              (else
                (Timeline|Door%20Opening%20Animation Reverse)))))))))

(event Input|TouchEvents|InputTouch
  (params (Location :type Vector) (FingerIndex :type ETouchIndex%20Enum))
  ;[1 1 1] Door
  (:Pressed
    (if (Utilities|Enum|Equal(Enum) FingerIndex "Touch1")
      (Utilities|FlowControl|Gate true
        (:Exit
          (if (Variables|Default|GetFakeDoor)
            (Utilities|FlowControl|DoOnce false
              (:Completed
                (Widget|SetVisibility (Variables|/Game/SimpleDoorLockSystem/UMG´s/FakeDoorText.FakeDoorText_C|GetTextBox (stale EventBeginPlay _returnvalue_2)) "Visible")
                (Utilities|FlowControl|Delay 3.0)
                (Widget|SetVisibility (Variables|/Game/SimpleDoorLockSystem/UMG´s/FakeDoorText.FakeDoorText_C|GetTextBox (stale EventBeginPlay _returnvalue_2)) "Hidden")
                (CallFunction|Reset2)))
            (elif (Variables|Default|GetLocked)
              (Utilities|FlowControl|DoOnce false
                (:Completed
                  (Rendering|Components|TextRender|SetText (Variables|/Game/SimpleDoorLockSystem/UMG´s/NeedKeyText.NeedKeyText_C|GetKeyText (stale EventBeginPlay _returnvalue)) "")
                  (Widget|SetVisibility (Variables|/Game/SimpleDoorLockSystem/UMG´s/NeedKeyText.NeedKeyText_C|GetHorizontalBox_428 (stale EventBeginPlay _returnvalue)) "Visible")
                  (Utilities|FlowControl|Delay 1.5)
                  (Widget|SetVisibility (Variables|/Game/SimpleDoorLockSystem/UMG´s/NeedKeyText.NeedKeyText_C|GetHorizontalBox_428 (stale EventBeginPlay _returnvalue)) "Hidden")
                  (CallFunction|Reset)))
              (elif (Variables|Default|GetClosed?)
                (bind _doorrotation (Timeline|Door%20Opening%20Animation Play)
                  (:Update
                    (Transformation|SetRelativeRotation (Variables|Default|GetDoor) (Math|Rotator|MakeRotator 0.0 0.0 _doorrotation) false false))
                  (:Finished
                    (Utilities|FlowControl|FlipFlop
                      (:A
                        (Variables|Default|SetClosed? false))
                      (:B
                        (Variables|Default|SetClosed? true)))))
                (else
                  (Timeline|Door%20Opening%20Animation Reverse))))))))))

(fn ConstructionScript)