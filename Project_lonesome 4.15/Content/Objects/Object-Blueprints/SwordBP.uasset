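; Sword pickup actor that the player collects with E or the gamepad bottom face button.
; Box overlap enables and disables the actor's input, so pickup only responds while overlapped.
; Pickup sets HasSword on MyGameInstance, appends SwordText to the character's log widget and hides the mesh with its collision off.
; A pickup text widget created at BeginPlay shows SwordText briefly before the actor destroys itself.
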(event OnComponentBeginOverlap(Box)
  (params (OverlappedComponent :type Primitive%20Component%20Object%20Reference) (OtherActor :type Actor%20Object%20Reference) (OtherComp :type Primitive%20Component%20Object%20Reference) (OtherBodyIndex :type Integer) (bFromSweep :type Boolean) (SweepResult :type Hit%20Result%20Structure%20%28by%20ref%29))
  (Input|EnableInput (Game|GetPlayerController 0)))

(event OnComponentEndOverlap(Box)
  (params (OverlappedComponent :type Primitive%20Component%20Object%20Reference) (OtherActor :type Actor%20Object%20Reference) (OtherComp :type Primitive%20Component%20Object%20Reference) (OtherBodyIndex :type Integer))
  (Input|DisableInput (Game|GetPlayerController 0)))

(event EventBeginPlay
  ;[1 1 1] Create Display Text Widget
  (bind _returnvalue (UserInterface|CreateWidget "/Game/Objects/Object-Blueprints/BP_PickUpText.BP_PickUpText_C"))
  (UserInterface|Viewport|AddtoViewport _returnvalue 0))

(event Input|KeyboardEvents|E
  (params (Key :type Key%20Structure :default "AnyKey"))
  (bind _staticmesh (Variables|Default|GetStaticMesh))
  (bind _swordtext (Variables|Default|GetSwordText))
  (:Pressed
    (bind _asmy_game_instance (Utilities|Casting|CastToMyGameInstance (Game|GetGameInstance)))
    (Variables|/Game/MyGameInstance.MyGameInstance_C|SetHasSword _asmy_game_instance (Class|KismetSystemLibrary|MakeLiteralBool true))
    (bind _asfirst_person_character (Utilities|Casting|CastToFirstPersonCharacter (Game|GetPlayerCharacter 0)))
    (Rendering|Components|TextRender|SetText (Variables|/Game/UI/Log.Log_C|GetMessageBox (Variables|/Game/FirstPersonBP/Blueprints/FirstPersonCharacter.FirstPersonCharacter_C|GetLog%20Referance _asfirst_person_character)) (Utilities|Text|ToText(String) (Utilities|String|Append (Utilities|String|ToString(Text) (Class|MultiLineEditableTextBox|GetText (Variables|/Game/UI/Log.Log_C|GetMessageBox (Variables|/Game/FirstPersonBP/Blueprints/FirstPersonCharacter.FirstPersonCharacter_C|GetLog%20Referance _asfirst_person_character)))) " 
" (Utilities|String|ToString(Text) _swordtext))))
    (Rendering|SetVisibility _staticmesh false false)
    (Collision|SetCollisionEnabled _staticmesh "NoCollision")
    (Rendering|Components|TextRender|SetText (Variables|/Game/Objects/Object-Blueprints/BP_PickUpText.BP_PickUpText_C|GetPickText (stale EventBeginPlay _returnvalue)) _swordtext)
    (Widget|SetVisibility (Variables|/Game/Objects/Object-Blueprints/BP_PickUpText.BP_PickUpText_C|GetHorizontalBox_0 (stale EventBeginPlay _returnvalue)) "Visible")
    (Utilities|FlowControl|Delay 3.0)
    (Widget|SetVisibility (Variables|/Game/Objects/Object-Blueprints/BP_PickUpText.BP_PickUpText_C|GetHorizontalBox_0 (stale EventBeginPlay _returnvalue)) "Hidden")
    (Actor|DestroyActor)))

(event Input|GamepadEvents|GamepadFaceButtonBottom
  (params (Key :type Key%20Structure :default "AnyKey"))
  (bind _staticmesh (Variables|Default|GetStaticMesh))
  (bind _swordtext (Variables|Default|GetSwordText))
  (:Pressed
    (bind _asmy_game_instance (Utilities|Casting|CastToMyGameInstance (Game|GetGameInstance)))
    (Variables|/Game/MyGameInstance.MyGameInstance_C|SetHasSword _asmy_game_instance (Class|KismetSystemLibrary|MakeLiteralBool true))
    (bind _asfirst_person_character (Utilities|Casting|CastToFirstPersonCharacter (Game|GetPlayerCharacter 0)))
    (Rendering|Components|TextRender|SetText (Variables|/Game/UI/Log.Log_C|GetMessageBox (Variables|/Game/FirstPersonBP/Blueprints/FirstPersonCharacter.FirstPersonCharacter_C|GetLog%20Referance _asfirst_person_character)) (Utilities|Text|ToText(String) (Utilities|String|Append (Utilities|String|ToString(Text) (Class|MultiLineEditableTextBox|GetText (Variables|/Game/UI/Log.Log_C|GetMessageBox (Variables|/Game/FirstPersonBP/Blueprints/FirstPersonCharacter.FirstPersonCharacter_C|GetLog%20Referance _asfirst_person_character)))) " 
" (Utilities|String|ToString(Text) _swordtext))))
    (Rendering|SetVisibility _staticmesh false false)
    (Collision|SetCollisionEnabled _staticmesh "NoCollision")
    (Rendering|Components|TextRender|SetText (Variables|/Game/Objects/Object-Blueprints/BP_PickUpText.BP_PickUpText_C|GetPickText (stale EventBeginPlay _returnvalue)) _swordtext)
    (Widget|SetVisibility (Variables|/Game/Objects/Object-Blueprints/BP_PickUpText.BP_PickUpText_C|GetHorizontalBox_0 (stale EventBeginPlay _returnvalue)) "Visible")
    (Utilities|FlowControl|Delay 3.0)
    (Widget|SetVisibility (Variables|/Game/Objects/Object-Blueprints/BP_PickUpText.BP_PickUpText_C|GetHorizontalBox_0 (stale EventBeginPlay _returnvalue)) "Hidden")
    (Actor|DestroyActor)))

(fn ConstructionScript)