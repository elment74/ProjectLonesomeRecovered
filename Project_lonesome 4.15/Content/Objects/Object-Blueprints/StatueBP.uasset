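; StatueBP is an interactable statue that can grant the Sapphire Eye and Circle Piece.
; Pressing E or the gamepad bottom face button checks HasRope on MyGameInstance and sets both item flags only if it is true.
; Either outcome appends its message to the player's log, shows it in a pickup widget created at BeginPlay, then hides the cube and destroys the actor after a delay.
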(event EventBeginPlay
  ;[1 1 1] Create Display Text Widget
  (bind _returnvalue (UserInterface|CreateWidget "/Game/Objects/Object-Blueprints/BP_PickUpText.BP_PickUpText_C"))
  (UserInterface|Viewport|AddtoViewport _returnvalue 0))

(event Input|KeyboardEvents|E
  (params (Key :type Key%20Structure :default "AnyKey"))
  (bind _returnvalue (Class|KismetSystemLibrary|MakeLiteralBool true))
  (bind _returnvalue_2 (Game|GetGameInstance))
  (bind _newvar_0 (Variables|Default|GetNewVar_0))
  (bind _cube (Variables|Default|GetCube))
  (bind _newvar_1 (Variables|Default|GetNewVar_1))
  (bind _cube_2 (Variables|Default|GetCube))
  (:Pressed
    (bind _asmy_game_instance (Utilities|Casting|CastToMyGameInstance _returnvalue_2))
    (if (Variables|/Game/MyGameInstance.MyGameInstance_C|GetHasRope _asmy_game_instance)
      (bind _asmy_game_instance_2 (Utilities|Casting|CastToMyGameInstance _returnvalue_2))
      (Variables|/Game/MyGameInstance.MyGameInstance_C|SetSapphireEye _asmy_game_instance_2 _returnvalue)
      (bind _asmy_game_instance_3 (Utilities|Casting|CastToMyGameInstance _returnvalue_2))
      (Variables|/Game/MyGameInstance.MyGameInstance_C|SetCirclePiece _asmy_game_instance_3 _returnvalue)
      (bind _asfirst_person_character (Utilities|Casting|CastToFirstPersonCharacter (Game|GetPlayerCharacter 0)))
      (Rendering|Components|TextRender|SetText (Variables|/Game/UI/Log.Log_C|GetMessageBox (Variables|/Game/FirstPersonBP/Blueprints/FirstPersonCharacter.FirstPersonCharacter_C|GetLog%20Referance _asfirst_person_character)) (Utilities|Text|ToText(String) (Utilities|String|Append (Utilities|String|ToString(Text) (Class|MultiLineEditableTextBox|GetText (Variables|/Game/UI/Log.Log_C|GetMessageBox (Variables|/Game/FirstPersonBP/Blueprints/FirstPersonCharacter.FirstPersonCharacter_C|GetLog%20Referance _asfirst_person_character)))) " 
" (Utilities|String|ToString(Text) _newvar_1))))
      (Rendering|SetVisibility _cube_2 false false)
      (Collision|SetCollisionEnabled _cube_2 "NoCollision")
      (Rendering|Components|TextRender|SetText (Variables|/Game/Objects/Object-Blueprints/BP_PickUpText.BP_PickUpText_C|GetPickText (stale EventBeginPlay _returnvalue)) _newvar_1)
      (Widget|SetVisibility (Variables|/Game/Objects/Object-Blueprints/BP_PickUpText.BP_PickUpText_C|GetHorizontalBox_0 (stale EventBeginPlay _returnvalue)) "Visible")
      (Utilities|FlowControl|Delay 3.0)
      (Widget|SetVisibility (Variables|/Game/Objects/Object-Blueprints/BP_PickUpText.BP_PickUpText_C|GetHorizontalBox_0 (stale EventBeginPlay _returnvalue)) "Hidden")
      (Actor|DestroyActor)
      (else
        (bind _asfirst_person_character_2 (Utilities|Casting|CastToFirstPersonCharacter (Game|GetPlayerCharacter 0)))
        (Rendering|Components|TextRender|SetText (Variables|/Game/UI/Log.Log_C|GetMessageBox (Variables|/Game/FirstPersonBP/Blueprints/FirstPersonCharacter.FirstPersonCharacter_C|GetLog%20Referance _asfirst_person_character_2)) (Utilities|Text|ToText(String) (Utilities|String|Append (Utilities|String|ToString(Text) (Class|MultiLineEditableTextBox|GetText (Variables|/Game/UI/Log.Log_C|GetMessageBox (Variables|/Game/FirstPersonBP/Blueprints/FirstPersonCharacter.FirstPersonCharacter_C|GetLog%20Referance _asfirst_person_character_2)))) "" (Utilities|String|ToString(Text) _newvar_0))))
        (Rendering|SetVisibility _cube false false)
        (Collision|SetCollisionEnabled _cube "NoCollision")
        (Rendering|Components|TextRender|SetText (Variables|/Game/Objects/Object-Blueprints/BP_PickUpText.BP_PickUpText_C|GetPickText (stale EventBeginPlay _returnvalue)) _newvar_0)
        (Widget|SetVisibility (Variables|/Game/Objects/Object-Blueprints/BP_PickUpText.BP_PickUpText_C|GetHorizontalBox_0 (stale EventBeginPlay _returnvalue)) "Visible")
        (Utilities|FlowControl|Delay 3.0)
        (Widget|SetVisibility (Variables|/Game/Objects/Object-Blueprints/BP_PickUpText.BP_PickUpText_C|GetHorizontalBox_0 (stale EventBeginPlay _returnvalue)) "Hidden")
        (Actor|DestroyActor)))))

(event Input|GamepadEvents|GamepadFaceButtonBottom
  (params (Key :type Key%20Structure :default "AnyKey"))
  (bind _returnvalue (Class|KismetSystemLibrary|MakeLiteralBool true))
  (bind _returnvalue_2 (Game|GetGameInstance))
  (bind _newvar_0 (Variables|Default|GetNewVar_0))
  (bind _cube (Variables|Default|GetCube))
  (bind _newvar_1 (Variables|Default|GetNewVar_1))
  (bind _cube_2 (Variables|Default|GetCube))
  (:Pressed
    (bind _asmy_game_instance (Utilities|Casting|CastToMyGameInstance _returnvalue_2))
    (if (Variables|/Game/MyGameInstance.MyGameInstance_C|GetHasRope _asmy_game_instance)
      (bind _asmy_game_instance_2 (Utilities|Casting|CastToMyGameInstance _returnvalue_2))
      (Variables|/Game/MyGameInstance.MyGameInstance_C|SetSapphireEye _asmy_game_instance_2 _returnvalue)
      (bind _asmy_game_instance_3 (Utilities|Casting|CastToMyGameInstance _returnvalue_2))
      (Variables|/Game/MyGameInstance.MyGameInstance_C|SetCirclePiece _asmy_game_instance_3 _returnvalue)
      (bind _asfirst_person_character (Utilities|Casting|CastToFirstPersonCharacter (Game|GetPlayerCharacter 0)))
      (Rendering|Components|TextRender|SetText (Variables|/Game/UI/Log.Log_C|GetMessageBox (Variables|/Game/FirstPersonBP/Blueprints/FirstPersonCharacter.FirstPersonCharacter_C|GetLog%20Referance _asfirst_person_character)) (Utilities|Text|ToText(String) (Utilities|String|Append (Utilities|String|ToString(Text) (Class|MultiLineEditableTextBox|GetText (Variables|/Game/UI/Log.Log_C|GetMessageBox (Variables|/Game/FirstPersonBP/Blueprints/FirstPersonCharacter.FirstPersonCharacter_C|GetLog%20Referance _asfirst_person_character)))) " 
" (Utilities|String|ToString(Text) _newvar_1))))
      (Rendering|SetVisibility _cube_2 false false)
      (Collision|SetCollisionEnabled _cube_2 "NoCollision")
      (Rendering|Components|TextRender|SetText (Variables|/Game/Objects/Object-Blueprints/BP_PickUpText.BP_PickUpText_C|GetPickText (stale EventBeginPlay _returnvalue)) _newvar_1)
      (Widget|SetVisibility (Variables|/Game/Objects/Object-Blueprints/BP_PickUpText.BP_PickUpText_C|GetHorizontalBox_0 (stale EventBeginPlay _returnvalue)) "Visible")
      (Utilities|FlowControl|Delay 3.0)
      (Widget|SetVisibility (Variables|/Game/Objects/Object-Blueprints/BP_PickUpText.BP_PickUpText_C|GetHorizontalBox_0 (stale EventBeginPlay _returnvalue)) "Hidden")
      (Actor|DestroyActor)
      (else
        (bind _asfirst_person_character_2 (Utilities|Casting|CastToFirstPersonCharacter (Game|GetPlayerCharacter 0)))
        (Rendering|Components|TextRender|SetText (Variables|/Game/UI/Log.Log_C|GetMessageBox (Variables|/Game/FirstPersonBP/Blueprints/FirstPersonCharacter.FirstPersonCharacter_C|GetLog%20Referance _asfirst_person_character_2)) (Utilities|Text|ToText(String) (Utilities|String|Append (Utilities|String|ToString(Text) (Class|MultiLineEditableTextBox|GetText (Variables|/Game/UI/Log.Log_C|GetMessageBox (Variables|/Game/FirstPersonBP/Blueprints/FirstPersonCharacter.FirstPersonCharacter_C|GetLog%20Referance _asfirst_person_character_2)))) "" (Utilities|String|ToString(Text) _newvar_0))))
        (Rendering|SetVisibility _cube false false)
        (Collision|SetCollisionEnabled _cube "NoCollision")
        (Rendering|Components|TextRender|SetText (Variables|/Game/Objects/Object-Blueprints/BP_PickUpText.BP_PickUpText_C|GetPickText (stale EventBeginPlay _returnvalue)) _newvar_0)
        (Widget|SetVisibility (Variables|/Game/Objects/Object-Blueprints/BP_PickUpText.BP_PickUpText_C|GetHorizontalBox_0 (stale EventBeginPlay _returnvalue)) "Visible")
        (Utilities|FlowControl|Delay 3.0)
        (Widget|SetVisibility (Variables|/Game/Objects/Object-Blueprints/BP_PickUpText.BP_PickUpText_C|GetHorizontalBox_0 (stale EventBeginPlay _returnvalue)) "Hidden")
        (Actor|DestroyActor)))))

(fn ConstructionScript)