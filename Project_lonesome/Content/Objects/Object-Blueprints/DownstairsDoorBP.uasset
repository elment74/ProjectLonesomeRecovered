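; A downstairs door Blueprint that moves the player to the First-Floor level when they hold the staircase key.
; Overlapping its Box enables player input on the actor and leaving disables it, so pressing E only works near the door.
; E reads the StaircaseKey flag from MyGameInstance and either opens the level or prints a placeholder message for the locked case.
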(event OnComponentBeginOverlap(Box)
  (params (OverlappedComponent :type Primitive%20Component%20Object%20Reference) (OtherActor :type Actor%20Object%20Reference) (OtherComp :type Primitive%20Component%20Object%20Reference) (OtherBodyIndex :type Integer) (bFromSweep :type Boolean) (SweepResult :type Hit%20Result%20Structure%20%28by%20ref%29))
  (Input|EnableInput (Game|GetPlayerController 0)))

(event OnComponentEndOverlap(Box)
  (params (OverlappedComponent :type Primitive%20Component%20Object%20Reference) (OtherActor :type Actor%20Object%20Reference) (OtherComp :type Primitive%20Component%20Object%20Reference) (OtherBodyIndex :type Integer))
  (Input|DisableInput (Game|GetPlayerController 0)))

(event Input|KeyboardEvents|E
  (params (Key :type Key%20Structure :default "AnyKey"))
  (:Pressed
    (bind _asmy_game_instance (Utilities|Casting|CastToMyGameInstance (Game|GetGameInstance)))
    (Variables|/Game/MyGameInstance.MyGameInstance_C|SetStaircaseKey _asmy_game_instance (Variables|/Game/MyGameInstance.MyGameInstance_C|GetStaircaseKey _asmy_game_instance))
    (if (Variables|/Game/MyGameInstance.MyGameInstance_C|GetStaircaseKey _asmy_game_instance)
      (Game|OpenLevel(byName) "First-Floor")
      (else
        (Development|PrintString "Add message saying unable to move to next level")))))

(fn ConstructionScript)