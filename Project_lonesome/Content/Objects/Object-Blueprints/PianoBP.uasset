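; PianoBP is an interactable piano puzzle that takes E input while an actor overlaps its Box.
; The first press flags the string as broken; later presses check the MyGameInstance flags for a replacement string, then a book of songs.
; With both items it sets Key7 true.
; Every press shows a matching message in a BP_PickUpText widget created at BeginPlay, hidden after a short delay.
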(event OnComponentBeginOverlap(Box)
  (params (OverlappedComponent :type Primitive%20Component%20Object%20Reference) (OtherActor :type Actor%20Object%20Reference) (OtherComp :type Primitive%20Component%20Object%20Reference) (OtherBodyIndex :type Integer) (bFromSweep :type Boolean) (SweepResult :type Hit%20Result%20Structure%20%28by%20ref%29))
  (Input|EnableInput (Game|GetPlayerController 0)))

(event OnComponentEndOverlap(Box)
  (params (OverlappedComponent :type Primitive%20Component%20Object%20Reference) (OtherActor :type Actor%20Object%20Reference) (OtherComp :type Primitive%20Component%20Object%20Reference) (OtherBodyIndex :type Integer))
  (Input|DisableInput (Game|GetPlayerController 0)))

(event EventBeginPlay
  ;[1 1 1] Create Display Text Widget
  (bind _returnvalue (UserInterface|CreateWidget "/Game/Objects/Object-Blueprints/BP_PickUpText.BP_PickUpText_C"))
  (UserInterface|Viewport|AddtoViewport _returnvalue 0))

(event Input|KeyboardEvents|E
  (params (Key :type Key%20Structure :default "AnyKey"))
  (bind _returnvalue (Game|GetGameInstance))
  (:Pressed
    (bind _asmy_game_instance (Utilities|Casting|CastToMyGameInstance _returnvalue))
    (if (Variables|/Game/MyGameInstance.MyGameInstance_C|GetBrokenPianoString _asmy_game_instance)
      (bind _asmy_game_instance_2 (Utilities|Casting|CastToMyGameInstance _returnvalue))
      (if (Variables|/Game/MyGameInstance.MyGameInstance_C|GetHasPianoString _asmy_game_instance_2)
        (bind _asmy_game_instance_3 (Utilities|Casting|CastToMyGameInstance _returnvalue))
        (if (Variables|/Game/MyGameInstance.MyGameInstance_C|GetHasBookOfSongs _asmy_game_instance_3)
          (bind _asmy_game_instance_4 (Utilities|Casting|CastToMyGameInstance (Game|GetGameInstance)))
          (Variables|/Game/MyGameInstance.MyGameInstance_C|SetKey%207 _asmy_game_instance_4 (Class|KismetSystemLibrary|MakeLiteralBool true))
          (Rendering|Components|TextRender|SetText (Variables|/Game/Objects/Object-Blueprints/BP_PickUpText.BP_PickUpText_C|GetPickText (stale EventBeginPlay _returnvalue)) (Variables|Default|GetHasSongBook))
          (else
            (Rendering|Components|TextRender|SetText (Variables|/Game/Objects/Object-Blueprints/BP_PickUpText.BP_PickUpText_C|GetPickText (stale EventBeginPlay _returnvalue)) (Variables|Default|GetNoSongBook))))
        (else
          (Rendering|Components|TextRender|SetText (Variables|/Game/Objects/Object-Blueprints/BP_PickUpText.BP_PickUpText_C|GetPickText (stale EventBeginPlay _returnvalue)) (Variables|Default|GetNeedNewString))))
      (else
        (Variables|/Game/MyGameInstance.MyGameInstance_C|SetBrokenPianoString _asmy_game_instance (Class|KismetSystemLibrary|MakeLiteralBool true))
        (Rendering|Components|TextRender|SetText (Variables|/Game/Objects/Object-Blueprints/BP_PickUpText.BP_PickUpText_C|GetPickText (stale EventBeginPlay _returnvalue)) (Variables|Default|GetBrokenString))))
    (Widget|SetVisibility (Variables|/Game/Objects/Object-Blueprints/BP_PickUpText.BP_PickUpText_C|GetHorizontalBox_0 (stale EventBeginPlay _returnvalue)) "Visible")
    (Utilities|FlowControl|Delay 3.0)
    (Widget|SetVisibility (Variables|/Game/Objects/Object-Blueprints/BP_PickUpText.BP_PickUpText_C|GetHorizontalBox_0 (stale EventBeginPlay _returnvalue)) "Hidden")))

(fn ConstructionScript)