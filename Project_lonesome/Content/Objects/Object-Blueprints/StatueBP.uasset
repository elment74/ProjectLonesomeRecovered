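; StatueBP is an interactive statue object that grants puzzle items to a player carrying rope.
; Pressing E checks the HasRope flag on MyGameInstance, then sets the SapphireEye and CirclePiece flags there.
; Without rope it prints a hint that rope is needed to reach something above.
; The key handler has no proximity or repeat check, and feedback uses PrintString only.
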(event Input|KeyboardEvents|E
  (params (Key :type Key%20Structure :default "AnyKey"))
  (bind _returnvalue (Class|KismetSystemLibrary|MakeLiteralBool true))
  (bind _returnvalue_2 (Game|GetGameInstance))
  (:Pressed
    (bind _asmy_game_instance (Utilities|Casting|CastToMyGameInstance _returnvalue_2))
    (if (Variables|/Game/MyGameInstance.MyGameInstance_C|GetHasRope _asmy_game_instance)
      (bind _asmy_game_instance_2 (Utilities|Casting|CastToMyGameInstance _returnvalue_2))
      (Variables|/Game/MyGameInstance.MyGameInstance_C|SetSapphireEye _asmy_game_instance_2 _returnvalue)
      (bind _asmy_game_instance_3 (Utilities|Casting|CastToMyGameInstance _returnvalue_2))
      (Variables|/Game/MyGameInstance.MyGameInstance_C|SetCirclePiece _asmy_game_instance_3 _returnvalue)
      (Development|PrintString "Player has stuff yay")
      (else
        (Development|PrintString "Looks like there is something up there I can get, if only I had some rope")))))

(fn ConstructionScript)