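; Interactive piano puzzle that advances a song quest and ultimately sets the Key7 flag.
; A box overlap toggles input, so nearby players interact with E or the gamepad bottom face button.
; Each press walks GameInstance flags: discover the broken string, require a replacement and songbook, then set half song, then full song.
; Every outcome appends to the character's message log and briefly shows a pickup text widget.
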(event OnComponentBeginOverlap(Box)
  (params (OverlappedComponent :type Primitive%20Component%20Object%20Reference) (OtherActor :type Actor%20Object%20Reference) (OtherComp :type Primitive%20Component%20Object%20Reference) (OtherBodyIndex :type Integer) (bFromSweep :type Boolean) (SweepResult :type Hit%20Result%20Structure%20%28by%20ref%29))
  (Input|EnableInput (Game|GetPlayerController 0)))

(event OnComponentEndOverlap(Box)
  (params (OverlappedComponent :type Primitive%20Component%20Object%20Reference) (OtherActor :type Actor%20Object%20Reference) (OtherComp :type Primitive%20Component%20Object%20Reference) (OtherBodyIndex :type Integer))
  (Input|DisableInput (Game|GetPlayerController 0)))

(event EventBeginPlay
  ;[1 1 1] Create Display Text Widget
  (bind _returnvalue (UserInterface|CreateWidget "/Game/Objects/Object-Blueprints/BP_PickUpText.BP_PickUpText_C"))
  (UserInterface|Viewport|AddtoViewport _returnvalue 0))

(event Input|KeyboardEvents|E
  (params (Key :type Key%20Structure :default "AnyKey"))
  (bind _returnvalue (Game|GetGameInstance))
  (bind _returnvalue_2 (Class|KismetSystemLibrary|MakeLiteralBool true))
  (bind _returnvalue_3 (Game|GetGameInstance))
  (bind _songbookplease (Variables|Default|GetSongBookPlease))
  (bind _hassongbook (Variables|Default|GetHasSongBook))
  (bind _brokenstring (Variables|Default|GetBrokenString))
  (bind _neednewstring (Variables|Default|GetNeedNewString))
  (:Pressed
    (bind _asmy_game_instance (Utilities|Casting|CastToMyGameInstance _returnvalue_3))
    (if (Variables|/Game/MyGameInstance.MyGameInstance_C|GetBrokenPianoString _asmy_game_instance)
      (bind _asmy_game_instance_2 (Utilities|Casting|CastToMyGameInstance _returnvalue_3))
      (if (Variables|/Game/MyGameInstance.MyGameInstance_C|GetHasPianoString _asmy_game_instance_2)
        (bind _asmy_game_instance_3 (Utilities|Casting|CastToMyGameInstance _returnvalue_3))
        (if (Variables|/Game/MyGameInstance.MyGameInstance_C|GetHasBookOfSongs _asmy_game_instance_3)
          (bind _asmy_game_instance_4 (Utilities|Casting|CastToMyGameInstance _returnvalue))
          (if (Variables|/Game/MyGameInstance.MyGameInstance_C|GetHalfSong _asmy_game_instance_4)
            (Variables|/Game/MyGameInstance.MyGameInstance_C|SetKey%207 _asmy_game_instance_4 _returnvalue_2)
            (Variables|/Game/MyGameInstance.MyGameInstance_C|SetFullSong _asmy_game_instance_4 _returnvalue_2)
            (bind _asfirst_person_character (Utilities|Casting|CastToFirstPersonCharacter (Game|GetPlayerCharacter 0)))
            (Rendering|Components|TextRender|SetText (Variables|/Game/UI/Log.Log_C|GetMessageBox (Variables|/Game/FirstPersonBP/Blueprints/FirstPersonCharacter.FirstPersonCharacter_C|GetLog%20Referance _asfirst_person_character)) (Utilities|Text|ToText(String) (Utilities|String|Append (Utilities|String|ToString(Text) (Class|MultiLineEditableTextBox|GetText (Variables|/Game/UI/Log.Log_C|GetMessageBox (Variables|/Game/FirstPersonBP/Blueprints/FirstPersonCharacter.FirstPersonCharacter_C|GetLog%20Referance _asfirst_person_character)))) " 
" (Utilities|String|ToString(Text) _hassongbook))))
            (Rendering|Components|TextRender|SetText (Variables|/Game/Objects/Object-Blueprints/BP_PickUpText.BP_PickUpText_C|GetPickText (stale EventBeginPlay _returnvalue)) _hassongbook)
            (else
              (bind _asmy_game_instance_5 (Utilities|Casting|CastToMyGameInstance _returnvalue))
              (Variables|/Game/MyGameInstance.MyGameInstance_C|SetHalfSong _asmy_game_instance_5 (Class|KismetSystemLibrary|MakeLiteralBool true))
              (bind _asfirst_person_character_2 (Utilities|Casting|CastToFirstPersonCharacter (Game|GetPlayerCharacter 0)))
              (Rendering|Components|TextRender|SetText (Variables|/Game/UI/Log.Log_C|GetMessageBox (Variables|/Game/FirstPersonBP/Blueprints/FirstPersonCharacter.FirstPersonCharacter_C|GetLog%20Referance _asfirst_person_character_2)) (Utilities|Text|ToText(String) (Utilities|String|Append (Utilities|String|ToString(Text) (Class|MultiLineEditableTextBox|GetText (Variables|/Game/UI/Log.Log_C|GetMessageBox (Variables|/Game/FirstPersonBP/Blueprints/FirstPersonCharacter.FirstPersonCharacter_C|GetLog%20Referance _asfirst_person_character_2)))) " 
" (Utilities|String|ToString(Text) (Variables|Default|GetHalfSong)))))
              (Rendering|Components|TextRender|SetText (Variables|/Game/Objects/Object-Blueprints/BP_PickUpText.BP_PickUpText_C|GetPickText (stale EventBeginPlay _returnvalue)) (Variables|Default|GetHalfSong))))
          (else
            (bind _asfirst_person_character_3 (Utilities|Casting|CastToFirstPersonCharacter (Game|GetPlayerCharacter 0)))
            (Rendering|Components|TextRender|SetText (Variables|/Game/UI/Log.Log_C|GetMessageBox (Variables|/Game/FirstPersonBP/Blueprints/FirstPersonCharacter.FirstPersonCharacter_C|GetLog%20Referance _asfirst_person_character_3)) (Utilities|Text|ToText(String) (Utilities|String|Append (Utilities|String|ToString(Text) (Class|MultiLineEditableTextBox|GetText (Variables|/Game/UI/Log.Log_C|GetMessageBox (Variables|/Game/FirstPersonBP/Blueprints/FirstPersonCharacter.FirstPersonCharacter_C|GetLog%20Referance _asfirst_person_character_3)))) " 
" (Utilities|String|ToString(Text) _songbookplease))))
            (Rendering|Components|TextRender|SetText (Variables|/Game/Objects/Object-Blueprints/BP_PickUpText.BP_PickUpText_C|GetPickText (stale EventBeginPlay _returnvalue)) _songbookplease)))
        (else
          (bind _asfirst_person_character_4 (Utilities|Casting|CastToFirstPersonCharacter (Game|GetPlayerCharacter 0)))
          (Rendering|Components|TextRender|SetText (Variables|/Game/UI/Log.Log_C|GetMessageBox (Variables|/Game/FirstPersonBP/Blueprints/FirstPersonCharacter.FirstPersonCharacter_C|GetLog%20Referance _asfirst_person_character_4)) (Utilities|Text|ToText(String) (Utilities|String|Append (Utilities|String|ToString(Text) (Class|MultiLineEditableTextBox|GetText (Variables|/Game/UI/Log.Log_C|GetMessageBox (Variables|/Game/FirstPersonBP/Blueprints/FirstPersonCharacter.FirstPersonCharacter_C|GetLog%20Referance _asfirst_person_character_4)))) " 
" (Utilities|String|ToString(Text) _neednewstring))))
          (Rendering|Components|TextRender|SetText (Variables|/Game/Objects/Object-Blueprints/BP_PickUpText.BP_PickUpText_C|GetPickText (stale EventBeginPlay _returnvalue)) _neednewstring)))
      (else
        (Variables|/Game/MyGameInstance.MyGameInstance_C|SetBrokenPianoString _asmy_game_instance (Class|KismetSystemLibrary|MakeLiteralBool true))
        (bind _asfirst_person_character_5 (Utilities|Casting|CastToFirstPersonCharacter (Game|GetPlayerCharacter 0)))
        (Rendering|Components|TextRender|SetText (Variables|/Game/UI/Log.Log_C|GetMessageBox (Variables|/Game/FirstPersonBP/Blueprints/FirstPersonCharacter.FirstPersonCharacter_C|GetLog%20Referance _asfirst_person_character_5)) (Utilities|Text|ToText(String) (Utilities|String|Append (Utilities|String|ToString(Text) (Class|MultiLineEditableTextBox|GetText (Variables|/Game/UI/Log.Log_C|GetMessageBox (Variables|/Game/FirstPersonBP/Blueprints/FirstPersonCharacter.FirstPersonCharacter_C|GetLog%20Referance _asfirst_person_character_5)))) " 
" (Utilities|String|ToString(Text) _brokenstring))))
        (Rendering|Components|TextRender|SetText (Variables|/Game/Objects/Object-Blueprints/BP_PickUpText.BP_PickUpText_C|GetPickText (stale EventBeginPlay _returnvalue)) _brokenstring)))
    (Widget|SetVisibility (Variables|/Game/Objects/Object-Blueprints/BP_PickUpText.BP_PickUpText_C|GetHorizontalBox_0 (stale EventBeginPlay _returnvalue)) "Visible")
    (Utilities|FlowControl|Delay 3.0)
    (Widget|SetVisibility (Variables|/Game/Objects/Object-Blueprints/BP_PickUpText.BP_PickUpText_C|GetHorizontalBox_0 (stale EventBeginPlay _returnvalue)) "Hidden")))

(event Input|GamepadEvents|GamepadFaceButtonBottom
  (params (Key :type Key%20Structure :default "AnyKey"))
  (bind _returnvalue (Game|GetGameInstance))
  (bind _returnvalue_2 (Class|KismetSystemLibrary|MakeLiteralBool true))
  (bind _returnvalue_3 (Game|GetGameInstance))
  (bind _songbookplease (Variables|Default|GetSongBookPlease))
  (bind _hassongbook (Variables|Default|GetHasSongBook))
  (bind _brokenstring (Variables|Default|GetBrokenString))
  (bind _neednewstring (Variables|Default|GetNeedNewString))
  (:Pressed
    (bind _asmy_game_instance (Utilities|Casting|CastToMyGameInstance _returnvalue_3))
    (if (Variables|/Game/MyGameInstance.MyGameInstance_C|GetBrokenPianoString _asmy_game_instance)
      (bind _asmy_game_instance_2 (Utilities|Casting|CastToMyGameInstance _returnvalue_3))
      (if (Variables|/Game/MyGameInstance.MyGameInstance_C|GetHasPianoString _asmy_game_instance_2)
        (bind _asmy_game_instance_3 (Utilities|Casting|CastToMyGameInstance _returnvalue_3))
        (if (Variables|/Game/MyGameInstance.MyGameInstance_C|GetHasBookOfSongs _asmy_game_instance_3)
          (bind _asmy_game_instance_4 (Utilities|Casting|CastToMyGameInstance _returnvalue))
          (if (Variables|/Game/MyGameInstance.MyGameInstance_C|GetHalfSong _asmy_game_instance_4)
            (Variables|/Game/MyGameInstance.MyGameInstance_C|SetKey%207 _asmy_game_instance_4 _returnvalue_2)
            (Variables|/Game/MyGameInstance.MyGameInstance_C|SetFullSong _asmy_game_instance_4 _returnvalue_2)
            (bind _asfirst_person_character (Utilities|Casting|CastToFirstPersonCharacter (Game|GetPlayerCharacter 0)))
            (Rendering|Components|TextRender|SetText (Variables|/Game/UI/Log.Log_C|GetMessageBox (Variables|/Game/FirstPersonBP/Blueprints/FirstPersonCharacter.FirstPersonCharacter_C|GetLog%20Referance _asfirst_person_character)) (Utilities|Text|ToText(String) (Utilities|String|Append (Utilities|String|ToString(Text) (Class|MultiLineEditableTextBox|GetText (Variables|/Game/UI/Log.Log_C|GetMessageBox (Variables|/Game/FirstPersonBP/Blueprints/FirstPersonCharacter.FirstPersonCharacter_C|GetLog%20Referance _asfirst_person_character)))) " 
" (Utilities|String|ToString(Text) _hassongbook))))
            (Rendering|Components|TextRender|SetText (Variables|/Game/Objects/Object-Blueprints/BP_PickUpText.BP_PickUpText_C|GetPickText (stale EventBeginPlay _returnvalue)) _hassongbook)
            (else
              (bind _asmy_game_instance_5 (Utilities|Casting|CastToMyGameInstance _returnvalue))
              (Variables|/Game/MyGameInstance.MyGameInstance_C|SetHalfSong _asmy_game_instance_5 (Class|KismetSystemLibrary|MakeLiteralBool true))
              (bind _asfirst_person_character_2 (Utilities|Casting|CastToFirstPersonCharacter (Game|GetPlayerCharacter 0)))
              (Rendering|Components|TextRender|SetText (Variables|/Game/UI/Log.Log_C|GetMessageBox (Variables|/Game/FirstPersonBP/Blueprints/FirstPersonCharacter.FirstPersonCharacter_C|GetLog%20Referance _asfirst_person_character_2)) (Utilities|Text|ToText(String) (Utilities|String|Append (Utilities|String|ToString(Text) (Class|MultiLineEditableTextBox|GetText (Variables|/Game/UI/Log.Log_C|GetMessageBox (Variables|/Game/FirstPersonBP/Blueprints/FirstPersonCharacter.FirstPersonCharacter_C|GetLog%20Referance _asfirst_person_character_2)))) " 
" (Utilities|String|ToString(Text) (Variables|Default|GetHalfSong)))))
              (Rendering|Components|TextRender|SetText (Variables|/Game/Objects/Object-Blueprints/BP_PickUpText.BP_PickUpText_C|GetPickText (stale EventBeginPlay _returnvalue)) (Variables|Default|GetHalfSong))))
          (else
            (bind _asfirst_person_character_3 (Utilities|Casting|CastToFirstPersonCharacter (Game|GetPlayerCharacter 0)))
            (Rendering|Components|TextRender|SetText (Variables|/Game/UI/Log.Log_C|GetMessageBox (Variables|/Game/FirstPersonBP/Blueprints/FirstPersonCharacter.FirstPersonCharacter_C|GetLog%20Referance _asfirst_person_character_3)) (Utilities|Text|ToText(String) (Utilities|String|Append (Utilities|String|ToString(Text) (Class|MultiLineEditableTextBox|GetText (Variables|/Game/UI/Log.Log_C|GetMessageBox (Variables|/Game/FirstPersonBP/Blueprints/FirstPersonCharacter.FirstPersonCharacter_C|GetLog%20Referance _asfirst_person_character_3)))) " 
" (Utilities|String|ToString(Text) _songbookplease))))
            (Rendering|Components|TextRender|SetText (Variables|/Game/Objects/Object-Blueprints/BP_PickUpText.BP_PickUpText_C|GetPickText (stale EventBeginPlay _returnvalue)) _songbookplease)))
        (else
          (bind _asfirst_person_character_4 (Utilities|Casting|CastToFirstPersonCharacter (Game|GetPlayerCharacter 0)))
          (Rendering|Components|TextRender|SetText (Variables|/Game/UI/Log.Log_C|GetMessageBox (Variables|/Game/FirstPersonBP/Blueprints/FirstPersonCharacter.FirstPersonCharacter_C|GetLog%20Referance _asfirst_person_character_4)) (Utilities|Text|ToText(String) (Utilities|String|Append (Utilities|String|ToString(Text) (Class|MultiLineEditableTextBox|GetText (Variables|/Game/UI/Log.Log_C|GetMessageBox (Variables|/Game/FirstPersonBP/Blueprints/FirstPersonCharacter.FirstPersonCharacter_C|GetLog%20Referance _asfirst_person_character_4)))) " 
" (Utilities|String|ToString(Text) _neednewstring))))
          (Rendering|Components|TextRender|SetText (Variables|/Game/Objects/Object-Blueprints/BP_PickUpText.BP_PickUpText_C|GetPickText (stale EventBeginPlay _returnvalue)) _neednewstring)))
      (else
        (Variables|/Game/MyGameInstance.MyGameInstance_C|SetBrokenPianoString _asmy_game_instance (Class|KismetSystemLibrary|MakeLiteralBool true))
        (bind _asfirst_person_character_5 (Utilities|Casting|CastToFirstPersonCharacter (Game|GetPlayerCharacter 0)))
        (Rendering|Components|TextRender|SetText (Variables|/Game/UI/Log.Log_C|GetMessageBox (Variables|/Game/FirstPersonBP/Blueprints/FirstPersonCharacter.FirstPersonCharacter_C|GetLog%20Referance _asfirst_person_character_5)) (Utilities|Text|ToText(String) (Utilities|String|Append (Utilities|String|ToString(Text) (Class|MultiLineEditableTextBox|GetText (Variables|/Game/UI/Log.Log_C|GetMessageBox (Variables|/Game/FirstPersonBP/Blueprints/FirstPersonCharacter.FirstPersonCharacter_C|GetLog%20Referance _asfirst_person_character_5)))) " 
" (Utilities|String|ToString(Text) _brokenstring))))
        (Rendering|Components|TextRender|SetText (Variables|/Game/Objects/Object-Blueprints/BP_PickUpText.BP_PickUpText_C|GetPickText (stale EventBeginPlay _returnvalue)) _brokenstring)))
    (Widget|SetVisibility (Variables|/Game/Objects/Object-Blueprints/BP_PickUpText.BP_PickUpText_C|GetHorizontalBox_0 (stale EventBeginPlay _returnvalue)) "Visible")
    (Utilities|FlowControl|Delay 3.0)
    (Widget|SetVisibility (Variables|/Game/Objects/Object-Blueprints/BP_PickUpText.BP_PickUpText_C|GetHorizontalBox_0 (stale EventBeginPlay _returnvalue)) "Hidden")))

(fn ConstructionScript)