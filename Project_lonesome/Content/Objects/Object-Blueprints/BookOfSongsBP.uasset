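; Blueprint for the Book of Songs pickup, which the player collects by pressing E while near it.
; Overlapping its Box component enables input on the actor for the first player controller, and leaving the box disables it.
; Pressing E sets HasBookOfSongs to true on MyGameInstance, prints debug strings and destroys the actor.
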(event OnComponentBeginOverlap(Box)
  (params (OverlappedComponent :type Primitive%20Component%20Object%20Reference) (OtherActor :type Actor%20Object%20Reference) (OtherComp :type Primitive%20Component%20Object%20Reference) (OtherBodyIndex :type Integer) (bFromSweep :type Boolean) (SweepResult :type Hit%20Result%20Structure%20%28by%20ref%29))
  (Input|EnableInput (Game|GetPlayerController 0)))

(event OnComponentEndOverlap(Box)
  (params (OverlappedComponent :type Primitive%20Component%20Object%20Reference) (OtherActor :type Actor%20Object%20Reference) (OtherComp :type Primitive%20Component%20Object%20Reference) (OtherBodyIndex :type Integer))
  (Input|DisableInput (Game|GetPlayerController 0)))

(event Input|KeyboardEvents|E
  (params (Key :type Key%20Structure :default "AnyKey"))
  (bind _returnvalue (Class|KismetSystemLibrary|MakeLiteralBool true))
  (:Pressed
    (bind _asmy_game_instance (Utilities|Casting|CastToMyGameInstance (Game|GetGameInstance)))
    (Variables|/Game/MyGameInstance.MyGameInstance_C|SetHasBookOfSongs _asmy_game_instance _returnvalue)
    (Development|PrintString (Utilities|String|ToString(Boolean) _returnvalue))
    (Development|PrintString "deleted yet?")
    (Actor|DestroyActor)))

(fn ConstructionScript)